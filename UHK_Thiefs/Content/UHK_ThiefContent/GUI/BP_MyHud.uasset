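; HUD Blueprint for the UHK character that manages the main menu and health bar widgets.
; BeginPlay caches the player character, creates both widgets, and shows the health bar with the character's current HP.
; ShowHideMainMenu toggles the menu in the viewport.
; GetDamage and Heal step the character's HP by one, clamping only the value sent to the health bar, not the stored HP.
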(event `self.ReceiveBeginPlay`
  ;[1 1 1] Create widgets
  (`|ExecutionSequence`
    (:`then_0`
      (bind _asbp_uhkcharacter (cast `/Game/UHK_ThiefContent/Player/BP_UHKCharacter` (`GameplayStatics.GetPlayerCharacter` 0)))
      (set `self.Character` _asbp_uhkcharacter))
    (:`then_1`
      ;;[1 1 1] Create Main menu
      (bind _returnvalue (`|CreateWidget` "/Game/UHK_ThiefContent/GUI/BPW_MainMenu.BPW_MainMenu_C"))
      (set `self.MyMenu` _returnvalue))
    (:`then_2`
      ;;[1 1 1] Create and set health
      (bind _returnvalue_2 (`|CreateWidget` "/Game/UHK_ThiefContent/GUI/BPW_HealthBar.BPW_HealthBar_C"))
      (bind _output_get (set `self.HealthBar` _returnvalue_2))
      (`UserWidget.AddToViewport` _output_get 0)
      (`/Game/UHK_ThiefContent/GUI/BPW_HealthBar.SetHealth` _output_get (`/Game/UHK_ThiefContent/Player/BP_UHKCharacter.HP_Current` (`self.Character`))))))

(event `ShowHideMainMenu`
  (bind _mymenu (`self.MyMenu`))
  ;[1 1 1] Show or hide main menu
  (if (`Widget.IsVisible` (`self.MyMenu`))
    (`Widget.RemoveFromParent` _mymenu)
    (else
      (`UserWidget.AddToViewport` _mymenu 0))))

(event `GetDamage`
  (bind _character (`self.Character`))
  ;[1 1 1] Change in health
  (bind _result (`/Engine/EditorBlueprintResources/StandardMacros.DecrementInt` (`/Game/UHK_ThiefContent/Player/BP_UHKCharacter.HP_Current` _character))
    (:`  `
      (`/Game/UHK_ThiefContent/GUI/BPW_HealthBar.UpdateHealth` (`self.HealthBar`) (`KismetMathLibrary.Clamp` _result 0 (`/Game/UHK_ThiefContent/Player/BP_UHKCharacter.HP_Max` _character))))))

(event `Heal`
  (bind _character (`self.Character`))
  ;[1 1 1] Change in health
  (bind _result (`/Engine/EditorBlueprintResources/StandardMacros.IncrementInt` (`/Game/UHK_ThiefContent/Player/BP_UHKCharacter.HP_Current` _character))
    (:`  `
      (`/Game/UHK_ThiefContent/GUI/BPW_HealthBar.UpdateHealth` (`self.HealthBar`) (`KismetMathLibrary.Clamp` _result 0 (`/Game/UHK_ThiefContent/Player/BP_UHKCharacter.HP_Max` _character))))))

(fn `UserConstructionScript`)